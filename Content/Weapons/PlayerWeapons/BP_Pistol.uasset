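; BP_Pistol is a player pistol weapon that adds firing feedback on top of its parent weapon class.
; StartFire runs the parent logic, calls PlayAnimation on the weapon mesh, spawns a muzzle flash at the jnt_MuzzleFlash socket and plays the 2D Foliage_Placed sound.
; StopFire and construction only call the parent.
; An attached-emitter variant of the muzzle flash is left unconnected.
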(event `self.StartFire`
  (bind _weaponmesh (`self.WeaponMesh`))
  (`parent.StartFire`)
  ;[1 1 1] WeaponAnimation if there is any
  (`SkeletalMeshComponent.PlayAnimation` (`self.WeaponMesh`) null false)
  (`GameplayStatics.SpawnEmitterAtLocation` "/Game/Weapons/FX/P_Lisa_Primary_MuzzleFlash.P_Lisa_Primary_MuzzleFlash" (`SceneComponent.GetSocketLocation` _weaponmesh "jnt_MuzzleFlash") (`SceneComponent.GetSocketRotation` _weaponmesh "jnt_MuzzleFlash"))
  (`GameplayStatics.PlaySound2D` "/Engine/VREditor/Sounds/UI/Foliage_Placed.Foliage_Placed"))

(event `self.StopFire`
  (`parent.StopFire`))

(fn `UserConstructionScript`
  (`parent.UserConstructionScript`))