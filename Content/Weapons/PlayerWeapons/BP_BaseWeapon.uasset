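; Base player weapon that fires projectiles automatically from StartFire until StopFire and tracks ammo in the WeaponInfo struct.
; A Gate looping through a retriggerable delay sets the fire rate, with each shot spending one round or printing an out-of-ammo message.
; CalculateShootInfo traces from the player camera and aims the muzzle-socket spawn at the hit or trace end, so shots converge on the view center.
; The construction script writes the weapon's class into WeaponInfo; older trace, spawn and muzzle-flash nodes remain disconnected.
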(event `self.ReceiveBeginPlay`)

(event `StartFire`
  (bind _weaponinfo (`self.WeaponInfo`))
  (`|ExecutionSequence`
    (:`then_0`
      (goto _label :!via `Open`))
    (:`then_1`
      (`/Engine/EditorBlueprintResources/StandardMacros.Gate` true :!label _label
        (:`Exit`
          (`|ExecutionSequence`
            (:`then_0`
              (`KismetSystemLibrary.RetriggerableDelay` 0.4)
              (goto _label))
            (:`then_1`
              (if (<= (`.CurrentAmmo_8_87898D7E473529B933E13388FFC9A916` (break `/Game/Weapons/PlayerWeapons/Struct_WeaponType` (`self.WeaponInfo`))) 0)
                (`KismetSystemLibrary.PrintString` "Out of Ammo" true true (struct :`R` 1.0 :`B` 0.091064 :`A` 1.0))
                (else
                  (bind _shoottolocation (`self.CalculateShootInfo`))
                  (`|SpawnActorFromClass` (`self.ProjectileClass`) _shoottolocation "AlwaysSpawn" "OverrideRootScale" null null)
                  (setmembers `/Game/Weapons/PlayerWeapons/Struct_WeaponType` :`StructRef` _weaponinfo :`CurrentAmmo` (- (`.CurrentAmmo_8_87898D7E473529B933E13388FFC9A916` (break `/Game/Weapons/PlayerWeapons/Struct_WeaponType` _weaponinfo)) 1)))))))))))

(event `StopFire`
  (goto _label :!via `Close`))

(fn `CalculateShootInfo`
  (returns (ShootToLocation :type "Transform Structure"))
  (bind _returnvalue (`SceneComponent.GetSocketLocation` (`self.WeaponMesh`) "jnt_MuzzleFlash"))
  (bind _camera (`/Game/PlayerCharacter/Lisa/Blueprints/BP_Lisa_Shooter.Camera` (`self.PlayerCharacter`)))
  (bind _returnvalue_2 (`SceneComponent.K2_GetComponentLocation` _camera))
  (bind _returnvalue_3 (+ _returnvalue_2 (* (`SceneComponent.GetForwardVector` _camera) 10000.0)))
  (bind (_outhit _returnvalue_4) (`KismetSystemLibrary.LineTraceSingle` _returnvalue_2 _returnvalue_3 "TraceTypeQuery3"))
  (if _returnvalue_4
    (return (`KismetMathLibrary.MakeTransform` _returnvalue (`KismetMathLibrary.FindLookAtRotation` _returnvalue (`.ImpactPoint` (`GameplayStatics.BreakHitResult` _outhit)))))
    (else
      (return (`KismetMathLibrary.MakeTransform` _returnvalue (`KismetMathLibrary.FindLookAtRotation` _returnvalue _returnvalue_3))))))

(fn `SetPlayerCharacter`
  (params (PlayerCharacter :type "/Game/PlayerCharacter/Lisa/Blueprints/BP_Lisa_Shooter Object Reference"))
  (set `self.PlayerCharacter` PlayerCharacter))

(fn `UserConstructionScript`
  (bind (_weaponinfo_itemtype _weaponinfo_itemclass _weaponinfo_currentammo _weaponinfo_maxammo _weaponinfo_damage _weaponinfo_itemimage _weaponinfo_equipsocketname _weaponinfo_unequipsocketname) (break `/Game/Weapons/PlayerWeapons/Struct_WeaponType` (`self.WeaponInfo`)))
  (set `self.WeaponInfo` (make `/Game/Weapons/PlayerWeapons/Struct_WeaponType` _weaponinfo_itemtype (`GameplayStatics.GetObjectClass` self) _weaponinfo_currentammo _weaponinfo_maxammo _weaponinfo_damage _weaponinfo_itemimage _weaponinfo_equipsocketname _weaponinfo_unequipsocketname)))